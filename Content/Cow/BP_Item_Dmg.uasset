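; Damage item pickup for the cow VR game, with a timeline-driven idle float that offsets the item's Z on each update.
; Overlapping its rocket collision flags the cow pawn as touching an item, sets the rocket power-up type and stores a reference to itself.
; GenerateCowpie and GenerateRocket, not called here, set the pawn's power-up type and spawn that weapon attached to its right-hand item socket.
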(event OnComponentBeginOverlap(RocketCollision)
  (params (OverlappedComponent :type Primitive%20Component%20Object%20Reference) (OtherActor :type Actor%20Object%20Reference) (OtherComp :type Primitive%20Component%20Object%20Reference) (OtherBodyIndex :type Integer) (bFromSweep :type Boolean) (SweepResult :type Hit%20Result%20Structure%20%28by%20ref%29))
  ;[0 0 0] Pick up rocket
  (bind _asbp_cow_vrpawn (Utilities|Casting|CastToBP_CowVRPawn OtherActor))
  (Variables|/Game/Cow/BP_CowVRPawn.BP_CowVRPawn_C|SethasTouchItem _asbp_cow_vrpawn true)
  (Variables|/Game/Cow/BP_CowVRPawn.BP_CowVRPawn_C|SetPowerUpItem _asbp_cow_vrpawn "NewEnumerator1")
  (Variables|/Game/Cow/BP_CowVRPawn.BP_CowVRPawn_C|SetItem_Rocket_Ref _asbp_cow_vrpawn self))

(event EventBeginPlay
  (bind _item (Variables|Default|Getitem))
  (bind _returnvalue (Transformation|GetWorldTransform _item))
  (bind (_x _y _z) (Math|Vector|BreakVector (.location _returnvalue)))
  ;[0 0 0] Idle Animation
  (bind _float (Timeline|Float_Anim Play)
    (:Update
      (Transformation|SetWorldLocation _item (Math|Vector|MakeVector _x _y (+ _float _z)) false false))))

(fn ConstructionScript)

(fn GenerateCowpie
  (params (CowPawn :type Object%20Object%20Reference))
  (bind _asbp_cow_vrpawn (Utilities|Casting|CastToBP_CowVRPawn CowPawn))
  (Variables|/Game/Cow/BP_CowVRPawn.BP_CowVRPawn_C|SetPowerUpItem _asbp_cow_vrpawn "NewEnumerator0")
  (bind _returnvalue (Game|SpawnActorfromClass "/Game/Cow/BP_Cow_Pie.BP_Cow_Pie_C" (Transformation|GetSocketTransform (Variables|/Game/Cow/BP_CowVRPawn.BP_CowVRPawn_C|GetCow_HandRight _asbp_cow_vrpawn) "Item_Socket" "RTS_World") "Undefined" "MultiplyWithRoot" 0 0))
  (Transformation|AttachComponentToComponent _returnvalue (Variables|/Game/Cow/BP_CowVRPawn.BP_CowVRPawn_C|GetCow_HandRight _asbp_cow_vrpawn) "Item_Socket" "SnapToTarget" "SnapToTarget" "SnapToTarget" true))

(fn GenerateRocket
  (params (CowPawn :type Object%20Object%20Reference))
  (bind _asbp_cow_vrpawn (Utilities|Casting|CastToBP_CowVRPawn CowPawn))
  (Variables|/Game/Cow/BP_CowVRPawn.BP_CowVRPawn_C|SetPowerUpItem _asbp_cow_vrpawn "NewEnumerator1")
  (bind _returnvalue (Game|SpawnActorfromClass "/Game/Cow/BP_RocketLauncher.BP_RocketLauncher_C" (Transformation|GetSocketTransform (Variables|/Game/Cow/BP_CowVRPawn.BP_CowVRPawn_C|GetCow_HandRight _asbp_cow_vrpawn) "Item_Socket" "RTS_World") "Undefined" "MultiplyWithRoot" 0 0))
  (Transformation|AttachComponentToComponent _returnvalue (Variables|/Game/Cow/BP_CowVRPawn.BP_CowVRPawn_C|GetCow_HandRight _asbp_cow_vrpawn) "Item_Socket" "SnapToTarget" "SnapToTarget" "SnapToTarget" true))