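; Desktop player pawn for the cow, handling UFO tractor-beam state, a rocket power-up and quitting on Escape.
; Each tick, the UFO's CaughtCow flag drives tractor-beam sphere visibility and zeroes DistanceMultiplier while caught.
; An overlap event matches the overlapped actor's class display name to BP_RocketLauncher, granting the power-up and revealing the launcher.
; Left click spends it, hiding the launcher and spawning a BP_Rocket at its transform.
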(event Custom|OnActorBeginOverlap_Event
  (params (OverlappedActor :type Actor%20Object%20Reference) (OtherActor :type Actor%20Object%20Reference))
  (if (Utilities|Enum|Equal(Enum) (Utilities|GetClassDisplayName (Utilities|GetClass OverlappedActor)) "BP_RocketLauncher")
    (Rendering|SetVisibility (Variables|Default|GetBP_RocketLauncher) true false)
    (Variables|Default|SetPowerUp "Rocket")))

(event EventTick
  (params (DeltaSeconds :type Float%20%28single-precision%29))
  (bind _ufo (Variables|Default|GetUFO))
  (bind _caughtcow (Variables|/Game/UFO/BP_UFODesktopPawn.BP_UFODesktopPawn_C|GetCaughtCow _ufo))
  (if _caughtcow
    (Variables|Default|SetDistanceMultiplier 0.0)
    (else
      (Variables|Default|SetDistanceMultiplier 6.0)))
  (Rendering|SetVisibility (Variables|Default|GetTractorBeamSphere) _caughtcow false))

(event Input|KeyboardEvents|Escape
  (params (Key :type Key%20Structure :default "None"))
  (:Pressed
    (Game|QuitGame 0 "Quit" false)))

(event Input|MouseEvents|LeftMouseButton
  (params (Key :type Key%20Structure :default "None"))
  (bind _bp_rocketlauncher (Variables|Default|GetBP_RocketLauncher))
  (:Pressed
    (if (Utilities|Enum|Equal(Enum) (Variables|Default|GetPowerUp) "Rocket")
      (Rendering|SetVisibility _bp_rocketlauncher false false)
      (Variables|Default|SetPowerUp "None")
      (Game|SpawnActorfromClass "/Game/Cow/BP_Rocket.BP_Rocket_C" (Transformation|GetWorldTransform _bp_rocketlauncher) "AlwaysSpawn" "MultiplyWithRoot" 0 0))))

(fn ConstructionScript)