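; BP_Item is a floating power-up pickup that gives the cow VR pawn an item.
; A looping or one-shot timeline offsets its height for the idle animation.
; On overlap, a pawn with HasTouchItem set has any held item reset, receives a cow pie attached to its right-hand socket, and the pickup destroys itself.
; GenerateRocket equips a rocket launcher likewise but is not called here.
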(event OnComponentBeginOverlap(CowpieCollision)
  (params (OverlappedComponent :type Primitive%20Component%20Object%20Reference) (OtherActor :type Actor%20Object%20Reference) (OtherComp :type Primitive%20Component%20Object%20Reference) (OtherBodyIndex :type Integer) (bFromSweep :type Boolean) (SweepResult :type Hit%20Result%20Structure%20%28by%20ref%29))
  ;[0 0 0] Pick up cowpie
  (bind _asbp_cow_vrpawn (Utilities|Casting|CastToBP_CowVRPawn OtherActor))
  (if (Variables|/Game/Cow/BP_CowVRPawn.BP_CowVRPawn_C|GethasTouchItem _asbp_cow_vrpawn)
    (Utilities|FlowControl|DoOnce false
      (:Completed
        ;;[0 0 0] Check if cow player has item on hand
        (bind _asbp_cow_vrpawn_2 (Utilities|Casting|CastToBP_CowVRPawn OtherActor))
        (if (Utilities|Enum|Equal(Enum) (Variables|/Game/Cow/BP_CowVRPawn.BP_CowVRPawn_C|GetPowerUpItem _asbp_cow_vrpawn_2) "NewEnumerator2")
          _
          (else
            ;;[0 0 0] Player has item, replace the item first. Then, generate new item
            (Default|ResetItemtoNull _asbp_cow_vrpawn_2)))
        ;;[0 0 0] Player doesn't have item
        (CallFunction|GenerateCowpie OtherActor)
        (Variables|/Game/Cow/BP_CowVRPawn.BP_CowVRPawn_C|SethasTouchItem _asbp_cow_vrpawn_2 false)
        (Actor|DestroyActor)))))

(event EventBeginPlay
  (bind _item (Variables|Default|GetItem))
  (bind _returnvalue (Transformation|GetWorldTransform _item))
  (bind (_x _y _z) (Math|Vector|BreakVector (.location _returnvalue)))
  ;[0 0 0] Idle Animation
  (bind _float (Timeline|Float_Anim Play)
    (:Update
      (Transformation|SetWorldLocation _item (Math|Vector|MakeVector _x _y (+ _float _z)) false false))))

(fn ConstructionScript)

(fn GenerateCowpie
  (params (CowPawn :type Object%20Object%20Reference))
  (bind _asbp_cow_vrpawn (Utilities|Casting|CastToBP_CowVRPawn CowPawn))
  (Variables|/Game/Cow/BP_CowVRPawn.BP_CowVRPawn_C|SetPowerUpItem _asbp_cow_vrpawn "NewEnumerator0")
  (bind _returnvalue (Game|SpawnActorfromClass "/Game/Cow/BP_Cow_Pie.BP_Cow_Pie_C" (Transformation|GetSocketTransform (Variables|/Game/Cow/BP_CowVRPawn.BP_CowVRPawn_C|GetHandRight _asbp_cow_vrpawn) "Item_Socket" "RTS_World") "Undefined" "MultiplyWithRoot" 0 0))
  (Transformation|AttachComponentToComponent _returnvalue (Variables|/Game/Cow/BP_CowVRPawn.BP_CowVRPawn_C|GetHandRight _asbp_cow_vrpawn) "Item_Socket" "SnapToTarget" "SnapToTarget" "SnapToTarget" true))

(fn GenerateRocket
  (params (CowPawn :type Object%20Object%20Reference))
  (bind _asbp_cow_vrpawn (Utilities|Casting|CastToBP_CowVRPawn CowPawn))
  (Variables|/Game/Cow/BP_CowVRPawn.BP_CowVRPawn_C|SetPowerUpItem _asbp_cow_vrpawn "NewEnumerator1")
  (bind _returnvalue (Game|SpawnActorfromClass "/Game/Cow/BP_RocketLauncher.BP_RocketLauncher_C" (Transformation|GetSocketTransform (Variables|/Game/Cow/BP_CowVRPawn.BP_CowVRPawn_C|GetHandRight _asbp_cow_vrpawn) "Item_Socket" "RTS_World") "Undefined" "MultiplyWithRoot" 0 0))
  (Transformation|AttachComponentToComponent _returnvalue (Variables|/Game/Cow/BP_CowVRPawn.BP_CowVRPawn_C|GetHandRight _asbp_cow_vrpawn) "Item_Socket" "SnapToTarget" "SnapToTarget" "SnapToTarget" true))