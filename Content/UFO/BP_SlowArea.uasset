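; BP_SlowArea is a UFO projectile that becomes an enlarged, temporary area, named as a slow area, where it lands.
; When its ground collision overlaps a Floor object, it stops its projectile movement, removes gravity and scales up the SlowArea component.
; After a delay it destroys itself through a ClientDestroy to ServerDestroy event chain.
; The graph contains no logic that applies a slow effect.
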(event OnComponentBeginOverlap(SlowAreaGroundCollision)
  (params (OverlappedComponent :type Primitive%20Component%20Object%20Reference) (OtherActor :type Actor%20Object%20Reference) (OtherComp :type Primitive%20Component%20Object%20Reference) (OtherBodyIndex :type Integer) (bFromSweep :type Boolean) (SweepResult :type Hit%20Result%20Structure%20%28by%20ref%29))
  (bind _projectilemovement (Variables|Default|GetProjectileMovement))
  (bind _slowarea (Variables|Default|GetSlowArea))
  (if (Utilities|Enum|Equal(Enum) (Utilities|String|EnumtoString (Collision|GetCollisionObjectType OtherComp)) "Floor")
    (Game|Components|ProjectileMovement|SetVelocityinLocalSpace _projectilemovement "0, 0, 0")
    (Variables|/Script/Engine.ProjectileMovementComponent|SetProjectileGravityScale _projectilemovement 0.0)
    (Transformation|SetWorldScale3D _slowarea (* (Transformation|GetWorldScale _slowarea) "8.000000,8.000000,8.000000"))
    (Utilities|FlowControl|Delay 8.0)
    (CallFunction|ClientDestroy)))

(event Custom|ClientDestroy
  (CallFunction|ServerDestroy))

(event Custom|ServerDestroy
  (Actor|DestroyActor))

(fn ConstructionScript)