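; Desktop-side UFO pawn with an energy-limited beam that flags CaughtCow when it hits the VR player's pawn.
; Each tick, a forward box trace from the camera runs while BeamOn, which is only cleared here, never set.
; Energy drains or recharges per frame, drives the beam light and widget progress bar, and cuts the beam below zero.
; Escape quits; the rocket hit check has no effect.
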(event Custom|OnActorHit_Event
  (params (SelfActor :type Actor%20Object%20Reference) (OtherActor :type Actor%20Object%20Reference) (NormalImpulse :type Vector) (Hit :type Hit%20Result%20Structure%20%28by%20ref%29))
  (if (Utilities|Enum|Equal(Enum) (Utilities|GetClassDisplayName (Utilities|GetClass OtherActor)) "BP_Rocket")
    _))

(event EventBeginPlay
  (Transformation|SetWorldLocation (Variables|Default|GetStaticMesh) (+ (Transformation|GetWorldLocation (Variables|Default|GetCamera)) "130.000000,0.000000,130.000000") false false)
  (bind _asbp_energy_widget (Utilities|Casting|CastToBP_EnergyWidget (UserInterface|GetUserWidgetObject (Variables|Default|GetWidget))))
  (Variables|Default|SetDisplayWidget _asbp_energy_widget))

(event EventTick
  (params (DeltaSeconds :type Float%20%28single-precision%29))
  (CallFunction|LaserHitSense)
  (CallFunction|EnergyManage))

(event Input|KeyboardEvents|Escape
  (params (Key :type Key%20Structure :default "None"))
  (:Pressed
    (Game|QuitGame 0 "Quit" false)))

(fn ConstructionScript)

(fn LaserHitSense
  (bind _camera (Variables|Default|GetCamera))
  (bind _returnvalue (Math|Vector|GetForwardVector _camera))
  (bind _returnvalue_2 (Transformation|GetWorldLocation _camera))
  (if (Variables|Default|GetBeamOn)
    (bind _outhit (Class|KismetSystemLibrary|BoxTraceSingleforObjects (+ _returnvalue_2 (* _returnvalue 4e+02)) (+ _returnvalue_2 (* _returnvalue 3e+04)) "60.000000,60.000000,60.000000" "0, 0, 0" (Utilities|Array|MakeArray "ObjectTypeQuery2" "ObjectTypeQuery1") false 0 "None" true))
    (if (Utilities|Enum|Equal(Enum) (Utilities|GetClassDisplayName (Utilities|GetClass (.HitActor (Collision|BreakHitResult _outhit)))) "VRPawn_C")
      (Variables|Default|SetCaughtCow true)
      (else
        (Variables|Default|SetCaughtCow false :!label _label)))
    (else
      (goto _label)))
  (return))

(fn EnergyManage
  (bind _beam (Variables|Default|GetBeam))
  (Progress|SetPercent (Variables|/Game/UFO/BP_EnergyWidget.BP_EnergyWidget_C|GetProgressBar_87 (Variables|Default|GetDisplayWidget)) (/ (Variables|Default|GetEnergyLevel) 1e+02))
  (if (Variables|Default|GetBeamOn)
    (Rendering|Components|Light|SetIntensity _beam 2e+05)
    (CallFunction|LaserHitSense)
    (Variables|Default|SetEnergyLevel (- (Variables|Default|GetEnergyLevel) 1.0))
    (else
      (Rendering|Components|Light|SetIntensity _beam 0.0)
      (if (< (Variables|Default|GetEnergyLevel) 1e+02)
        (Variables|Default|SetEnergyLevel (+ (Variables|Default|GetEnergyLevel) 1.0)))))
  (if (< (Variables|Default|GetEnergyLevel) 0.0)
    (Variables|Default|SetBeamOn false)))